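; TestPlayerBP is a test player Blueprint with a side-on camera that follows it in the Y-Z plane.
; BeginPlay shows the mouse cursor, and Tick moves the camera to the capsule's Y and Z, keeping its own X and a fixed rotation.
; An unconnected graph, which never runs, would tilt the capsule toward the cursor trace hit and flip its yaw by which side the hit is on.
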(event `self.ReceiveBeginPlay`
  (set `PlayerController.bShowMouseCursor` true (`GameplayStatics.GetPlayerController` 0)))

(event `self.ReceiveTick`
  (params (DeltaSeconds :type "Float (single-precision)"))
  (bind _camera (`self.Camera`))
  (`SceneComponent.K2_SetWorldLocationAndRotation` _camera (`KismetMathLibrary.MakeVector` (.x (`SceneComponent.K2_GetComponentLocation` _camera)) (.y (`SceneComponent.K2_GetComponentLocation` (`self.Capsule`))) (.z (`SceneComponent.K2_GetComponentLocation` (`self.Capsule`)))) (struct :`Yaw` 180.0) false false))

(fn `UserConstructionScript`)